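; BP_actorLight is an actor with a spot light that blinks a set number of times when play begins.
; The construction script hides the light, then BeginPlay loops through a Delay of Duration and a visibility toggle.
; A DoN gate set to twice Count ends the loop, giving Count on/off blinks that finish with the light off.
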(event `self.ReceiveBeginPlay`
  (`/Engine/EditorBlueprintResources/StandardMacros.Do N` (+ (`self.Count`) (`self.Count`)) :!label _label
    (:`Exit`
      (`KismetSystemLibrary.Delay` (`self.Duration`))
      (`SceneComponent.ToggleVisibility` (`self.SpotLight`) false)
      (goto _label))))

(fn `UserConstructionScript`
  (`SceneComponent.SetVisibility` (`self.SpotLight`) false false))